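; BPC_Base_Item is a base Blueprint for items that an interacting instigator can pick up.
; On Interaction, it checks the instigator for inventory space, then passes its ItemInfo through PickupMessage and destroys itself.
; The construction script runs the parent's, then rebuilds ItemInfo with the actor's own class written in, so the data passed on pickup identifies the class it came from.
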(event EventInteraction
  (params (Instigater :type CH%20My%20Character%20Object%20Reference))
  (if (Default|HasSpaceinInventory Instigater)
    (Class|BPIInteract|Pickup(Message) Instigater (Variables|Default|GetItem%20Info))
    (Actor|DestroyActor)))

(fn ConstructionScript
  (|CallParentFunction)
  (Variables|Default|SetItem%20Info (Utilities|Struct|MakeS_Item_Info (.itemtype (Variables|Default|GetItem%20Info)) (.itemname (Variables|Default|GetItem%20Info)) (.itemimage (Variables|Default|GetItem%20Info)) (Utilities|GetClass self) (.itemindex (Variables|Default|GetItem%20Info)) (.itemslot (Variables|Default|GetItem%20Info)) (.itemvalue (Variables|Default|GetItem%20Info)))))