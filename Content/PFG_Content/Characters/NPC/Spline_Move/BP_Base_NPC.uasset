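; Base NPC Blueprint for characters that move along a referenced spline.
; BeginPlay sets the speed to walk speed, and AddMovement advances the distance along the spline by speed, axis value and delta time.
; UpdateLocationAndRotation places the actor at that distance, taking X, Y and rotation from the spline but keeping its own Z.
; Neither movement function is called within this Blueprint.
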(event EventBeginPlay
  (Variables|Default|SetCharacter%20Speed (Variables|Default|GetWalk%20Speed)))

(fn ConstructionScript)

(fn AddMovement
  (bind _character_speed (Variables|Default|GetCharacter%20Speed))
  (bind _axis_value (Variables|Default|GetAxis%20Value))
  (bind _returnvalue (* _character_speed _axis_value))
  (Variables|Default|SetPlayer%20Acceleration _returnvalue)
  (Variables|Default|SetDistance%20Along%20Spline (+ (Variables|Default|GetDistance%20Along%20Spline) (* _returnvalue (Utilities|Time|GetWorldDeltaSeconds)))))

(fn UpdateLocationandRotation
  (bind _splineref (Variables|Default|GetSplineRef))
  (bind _distance_along_spline (Variables|Default|GetDistance%20Along%20Spline))
  (bind _spline (Variables|/Game/PFG_Content/Characters/NPC/Spline_Move/BP_Follow_Spline.BP_Follow_Spline_C|GetSpline _splineref))
  (bind _returnvalue (Spline|GetLocationatDistanceAlongSpline _spline _distance_along_spline "World"))
  (Transformation|SetActorLocationAndRotation (Math|Vector|MakeVector (.x _returnvalue) (.y _returnvalue) (.z (Transformation|GetActorLocation))) (Spline|GetRotationatDistanceAlongSpline (Variables|/Game/PFG_Content/Characters/NPC/Spline_Move/BP_Follow_Spline.BP_Follow_Spline_C|GetSpline (Variables|Default|GetSplineRef)) (Variables|Default|GetDistance%20Along%20Spline) "World")))